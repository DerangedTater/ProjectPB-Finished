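; Blueprint function library of static gameplay helpers for reaching ammo, weapon, character and combat components, factories and loadouts.
; Component getters call message functions on the passed actor, with only the ammo getter checking validity first.
; Factory and loadout getters cast the current game mode to PBGameMode, so they depend on that class being active.
; Ammo creation and data lookup by tag delegate to the ammo factory.
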(fn GetAmmoComponent
  (params (AmmoActor :type Actor%20Object%20Reference))
  (Utilities|IsValid AmmoActor
    (:Is%20Valid
      (bind _ammocomponent (Class|AmmoComponentInterface|GetAmmoComponent(Message) AmmoActor))
      (return _ammocomponent))))

(fn GetWeaponComponent
  (params (WeaponActor :type Actor%20Object%20Reference))
  (bind _weaponcomponent (Class|WeaponComponentInterface|GetWeaponComponent(Message) WeaponActor))
  (return _weaponcomponent))

(fn CreateAmmo
  (params (WorldContextObject :type Object%20Object%20Reference) (AmmoTag :type Gameplay%20Tag%20Structure))
  (bind _ammo (Default|CreateAmmo (CallFunction|GetAmmoFactory WorldContextObject) AmmoTag))
  (return _ammo))

(fn GetAmmoData
  (params (AmmoTag :type Gameplay%20Tag%20Structure))
  (bind (_bisvalid _ammodata) (Default|GetAmmoData (CallFunction|GetAmmoFactory) AmmoTag))
  (return _bisvalid _ammodata))

(fn GetCharacterFactory
  (bind _aspbgame_mode (Utilities|Casting|CastToPBGameMode (Game|GetGameMode)))
  (bind _characterfactory (Default|GetCharacterFactory _aspbgame_mode))
  (return _characterfactory))

(fn GetLoadout
  (params (LoadoutTag :type Gameplay%20Tag%20Structure))
  (bind _aspbgame_mode (Utilities|Casting|CastToPBGameMode (Game|GetGameMode)))
  (bind _loadoutdata (Default|GetLoadout _aspbgame_mode LoadoutTag))
  (return _loadoutdata))

(fn GetCombatSystemComponent
  (params (Actor :type Actor%20Object%20Reference))
  (bind _combatcomponent (Class|CombatComponentInterface|GetCombatComponent(Message) Actor))
  (return _combatcomponent))

(fn GetCharacterComponent
  (params (Actor :type Actor%20Object%20Reference))
  (bind _charactercomponent (Class|CharacterComponentInterface|GetCharacterComponent(Message) Actor))
  (return _charactercomponent))

(fn GetWeaponFactory
  (bind _aspbgame_mode (Utilities|Casting|CastToPBGameMode (Game|GetGameMode)))
  (bind _weaponfactory (Default|GetWeaponFactory _aspbgame_mode))
  (return _weaponfactory))

(fn GetAmmoFactory
  (bind _aspbgame_mode (Utilities|Casting|CastToPBGameMode (Game|GetGameMode)))
  (bind _ammofactory (Default|GetAmmoFactory _aspbgame_mode))
  (return _ammofactory))