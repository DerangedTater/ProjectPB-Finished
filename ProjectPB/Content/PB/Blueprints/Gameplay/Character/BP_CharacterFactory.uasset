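; BP_CharacterFactory is an actor that serves as a lookup cache for character data, keyed by character tag.
; On BeginPlay, CacheData reads every row of the composite data table DTComposite_Characters into the CharacterDataCached map under that row's CharacterTag.
; RetrieveCharacterData looks up a tag in that map and returns the data with a validity flag.
; Despite the Factory name, it spawns no characters itself.
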(event EventBeginPlay
  (CallFunction|CacheData))

(event Collision|EventActorBeginOverlap
  (params (OtherActor :type Actor%20Object%20Reference)))

(event EventTick
  (params (DeltaSeconds :type Float%20%28single-precision%29)))

(fn ConstructionScript)

(fn CacheData
  (bind _outrownames (DataTable|GetDataTableRowNames "/Game/PB/Data/Characters/DTComposite_Characters.DTComposite_Characters"))
  (for _array_element _outrownames
    (bind _returnvalue (Utilities|GetDataTableRow "/Game/PB/Data/Characters/DTComposite_Characters.DTComposite_Characters" _array_element)
      (:then
        (Utilities|Map|Add (Variables|Default|GetCharacterDataCached) (.CharacterTag (Utilities|Struct|BreakFCharacterData _returnvalue)) _returnvalue)))))

(fn RetrieveCharacterData
  (params (CharacterTag :type Gameplay%20Tag%20Structure))
  (bind _characterdatacached (Variables|Default|GetCharacterDataCached))
  (bind (_value _returnvalue) (Utilities|Map|Find _characterdatacached CharacterTag))
  (return _value _returnvalue))