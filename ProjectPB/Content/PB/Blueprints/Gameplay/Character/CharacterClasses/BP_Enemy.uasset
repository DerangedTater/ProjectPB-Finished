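; BP_Enemy is an enemy character Blueprint with an overhead-style status widget that is removed from the world when killed or zombified.
; Shortly after BeginPlay it creates a BP_CharacterListener, initializes it with itself and passes it to the BPW_Status widget.
; Each Tick it rotates the widget component to face the player's pawn.
; DoDeath and DoZombied run parent logic, then destroy the actor.
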(event EventBeginPlay
  (Utilities|FlowControl|Delay 0.5)
  (bind _asbpw_status (Utilities|Casting|CastToBPW_Status (UserInterface|GetUserWidgetObject (Variables|Default|GetStatus_Widget))))
  (bind _returnvalue (Game|ConstructObjectfromClass "/Game/PB/UI/BP_CharacterListener.BP_CharacterListener_C" self))
  (Default|Initialize _returnvalue self)
  (Default|ReceiveCharacterListener _asbpw_status _returnvalue))

(event EventTick
  (params (DeltaSeconds :type Float%20%28single-precision%29))
  (Transformation|SetWorldRotation (Variables|Default|GetStatus_Widget) (Math|Rotator|MakeRotfromX (- (Transformation|GetActorLocation (Pawn|GetControlledPawn (Game|GetPlayerController 0))) (Transformation|GetActorLocation))) false false))

(event EventDoZombied
  (|CallParentFunction)
  (Actor|DestroyActor))

(event EventDoDeath
  (|CallParentFunction)
  (Actor|DestroyActor))

(fn ConstructionScript)