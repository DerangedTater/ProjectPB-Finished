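; Character component that manages a character's stats, damage intake, death and reveal/conceal state.
; Setup pulls data by character type from the character factory, building tag-keyed BP_GameplayProperty stats, setting ammo multipliers and color scheme, and broadcasting loadouts.
; Damage adds flag-based ammo multipliers, is zeroed while concealed, and drains Shield before Health, though DamageValue passes zero to Health.
; Reveal-flagged damage exposes the character, optionally starting a timer.
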(fn InitStats
  (params (Stats :type Array%20of%20F%20Property%20Structures))
  (for _array_element Stats
    (bind _returnvalue (Game|ConstructObjectfromClass "/Game/PB/Blueprints/Gameplay/Properties/BP_GameplayProperty.BP_GameplayProperty_C" self))
    (Variables|/Game/PB/Blueprints/Gameplay/Properties/BP_Property.BP_Property_C|SetMax _returnvalue (.Max (Utilities|Struct|BreakFProperty _array_element)))
    (Variables|/Game/PB/Blueprints/Gameplay/Properties/BP_Property.BP_Property_C|SetRegenPerSecond _returnvalue 0.0)
    (Variables|/Game/PB/Blueprints/Gameplay/Properties/BP_Property.BP_Property_C|SetbMaxOnStart _returnvalue (.bStartAtMax (Utilities|Struct|BreakFProperty _array_element)))
    (Default|Initialize _returnvalue)
    (Utilities|Map|Add (Variables|Default|GetStats) (.PropertyTag (Utilities|Struct|BreakFProperty _array_element)) _returnvalue)))

(fn Damage
  (params (DamageObj :type BP%20Damage%20Object%20Reference))
  (bind _flag (Variables|/Game/PB/Blueprints/Gameplay/Damage/BP_Damage.BP_Damage_C|GetFlag DamageObj))
  (bind _ammodamagemultiplier (Variables|Default|GetAmmoDamageMultiplier))
  (bind (_value _returnvalue) (Utilities|Map|Find _ammodamagemultiplier _flag))
  (Default|CallOnPreDamage DamageObj)
  (Utilities|FlowControl|Sequence
    (:then_0
      (if _returnvalue
        (LocalVariables|SetLAmmoMultiplier _value)))
    (:then_1
      (if (not (Variables|Default|GetbRevealed))
        (LocalVariables|SetLRevealMultiplier 0.0)))
    (:then_2
      (if (== _flag "(TagName=\"Damage.Reveal\")")
        (CallFunction|Reveal)))
    (:then_3
      (bind _amountdamaged (CallFunction|DamageShield (* (* (Variables|/Game/PB/Blueprints/Gameplay/Damage/BP_Damage.BP_Damage_C|GetValue DamageObj) (+ (Variables|/Game/PB/Blueprints/Gameplay/Damage/BP_Damage.BP_Damage_C|GetMultiplier DamageObj) (LocalVariables|GetLAmmoMultiplier))) (LocalVariables|GetLRevealMultiplier))))
      (bind _amountapplied (CallFunction|DamageHealth (- (* (* (Variables|/Game/PB/Blueprints/Gameplay/Damage/BP_Damage.BP_Damage_C|GetValue DamageObj) (+ (Variables|/Game/PB/Blueprints/Gameplay/Damage/BP_Damage.BP_Damage_C|GetMultiplier DamageObj) (LocalVariables|GetLAmmoMultiplier))) (LocalVariables|GetLRevealMultiplier)) _amountdamaged)))
      (return (+ _amountdamaged _amountapplied)))))

(fn DamageShield
  (params (Amount :type Float%20%28single-precision%29))
  (bind _stats (Variables|Default|GetStats))
  (bind (_value _returnvalue) (Utilities|Map|Find _stats "(TagName=\"Character.Stat.Shield\")"))
  (if _returnvalue
    (bind _amounttaken (Default|Take _value Amount))
    (return _amounttaken)
    (else
      (return 0.0))))

(fn DamageHealth
  (params (Amount :type Float%20%28single-precision%29))
  (bind _stats (Variables|Default|GetStats))
  (bind (_value _returnvalue) (Utilities|Map|Find _stats "(TagName=\"Character.Stat.Health\")"))
  (if _returnvalue
    (bind _amounttaken (Default|Take _value Amount))
    (Utilities|FlowControl|Sequence
      (:then_0
        (if (<= (Variables|/Game/PB/Blueprints/Gameplay/Properties/BP_Property.BP_Property_C|GetCurrent _value) 0.0)
          (Default|CallOnDied)))
      (:then_1
        (return _amounttaken)))
    (else
      (return 0.0))))

(fn Reveal
  (bind _secondsuntilreconceal (Variables|Default|GetSecondsUntilReconceal))
  (if (not (Variables|Default|GetbRevealed))
    (Variables|Default|SetbRevealed true)
    (Default|CallOnRevealed)
    (if (> _secondsuntilreconceal 0.0)
      (Utilities|Time|SetTimerbyEvent (EventDispatchers|CreateEvent :!event Conceal) _secondsuntilreconceal))))

(fn Conceal
  (if (Variables|Default|GetbRevealed)
    (Variables|Default|SetbRevealed false)
    (Default|CallOnConcealed)))

(fn SetCharacterType
  (params (CharacterType :type Gameplay%20Tag%20Structure))
  (Variables|Default|SetCharacterType CharacterType)
  (if (not (Variables|Default|GetbInitialized))
    (CallFunction|SetupCharacter)
    (Variables|Default|SetbInitialized true)))

(fn SetupCharacter
  (bind _characterfactory (CallFunction|GetCharacterFactory))
  (Utilities|IsValid _characterfactory
    (:Is%20Valid
      (bind (_characterdata _bisvalid) (Default|RetrieveCharacterData _characterfactory (Variables|Default|GetCharacterType)))
      (if _bisvalid
        (bind _colorscheme (Class|ColorSchemeInterface|GetColor(Message) (Game|GetGameMode) (.colorscheme _characterdata)))
        (Variables|Default|SetAmmoDamageMultiplier (.damagemultipliers _characterdata))
        (Variables|Default|SetColorScheme _colorscheme)
        (CallFunction|InitStats (.stats _characterdata))
        (Default|CallOnReceivedLoadouts (.loadouts _characterdata))))))

(fn DamageValue
  (params (Value :type Float%20%28single-precision%29))
  (bind _amountdamaged (CallFunction|DamageShield Value))
  (bind _amountapplied (CallFunction|DamageHealth 0.0))
  (return (+ _amountdamaged _amountapplied)))