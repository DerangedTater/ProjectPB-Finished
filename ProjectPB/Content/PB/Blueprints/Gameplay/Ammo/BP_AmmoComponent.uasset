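; BP_AmmoComponent is an ammo component that holds a damage tag and value and produces damage objects from them.
; Initialize sets the tag and value, and Fire broadcasts OnFired.
; GetDamage constructs a BP_Damage with the owner as source and the owner's Instigator as instigator.
; It broadcasts OnPreDamage with that object before returning it, giving listeners a hook on each damage instance.
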(event EventBeginPlay)

(event EventTick
  (params (DeltaSeconds :type Float%20%28single-precision%29)))

(fn Fire
  (Default|CallOnFired))

(fn GetDamage
  (bind _returnvalue (Components|GetOwner))
  (bind _returnvalue_2 (Game|ConstructObjectfromClass "/Game/PB/Blueprints/Gameplay/Damage/BP_Damage.BP_Damage_C" self))
  (Default|Initialize _returnvalue_2 (Variables|/Script/Engine.Actor|GetInstigator _returnvalue) _returnvalue (Variables|Default|GetDamageTag) (Variables|Default|GetDamageValue) 1.0)
  (Default|CallOnPreDamage _returnvalue_2)
  (return _returnvalue_2))

(fn Initialize
  (params (DamageTag :type Gameplay%20Tag%20Structure) (DamageAmount :type Float%20%28single-precision%29))
  (Variables|Default|SetDamageTag DamageTag)
  (Variables|Default|SetDamageValue DamageAmount))