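; BP_AmmoFactory is an actor that spawns ammo actors by gameplay tag and serves ammo data lookups.
; On BeginPlay it caches DTComposite_Ammo rows into a map keyed by GameplayTag.
; CreateAmmo spawns the row's ammo class, applies game-mode colors via AmmoCosmeticInterface, and initializes and returns its ammo component with damage settings.
; Invalid tags or classes print an error, and spawned actors lacking a valid component are destroyed.
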(event EventBeginPlay
  (CallFunction|PopulateCache))

(event Collision|EventActorBeginOverlap
  (params (OtherActor :type Actor%20Object%20Reference)))

(event EventTick
  (params (DeltaSeconds :type Float%20%28single-precision%29)))

(fn ConstructionScript)

(fn PopulateCache
  (bind _outrownames (DataTable|GetDataTableRowNames "/Game/PB/Data/Ammo/DTComposite_Ammo.DTComposite_Ammo"))
  (for _array_element _outrownames
    (bind _returnvalue (Utilities|GetDataTableRow "/Game/PB/Data/Ammo/DTComposite_Ammo.DTComposite_Ammo" _array_element)
      (:then
        (Utilities|Map|Add (Variables|Default|GetAmmoData) (.GameplayTag (Utilities|Struct|BreakFAmmoData _returnvalue)) _returnvalue)))))

(fn CreateAmmo
  (params (AmmoTag :type Gameplay%20Tag%20Structure))
  (bind _ammodata (Variables|Default|GetAmmoData))
  (bind (_value _returnvalue) (Utilities|Map|Find _ammodata AmmoTag))
  (bind (_gameplaytag _ammotype _damagetag _basedamage _colorscheme) (Utilities|Struct|BreakFAmmoData _value))
  (bind _ammoclass (Utilities|GetClassDefaults _ammotype))
  (if _returnvalue
    (if (Utilities|IsValidClass _ammotype)
      (if (Utilities|IsValidClass _ammoclass)
        (bind _returnvalue_2 (Game|SpawnActorfromClass _ammoclass (Math|Transform|MakeTransform "0, 0, 0" "0, 0, 0" "1.000000,1,1") "AlwaysSpawn" 0 0))
        (Utilities|FlowControl|Sequence
          (:then_0
            (bind _asammo_cosmetic_interface (Utilities|Casting|CastToAmmoCosmeticInterface _returnvalue_2))
            (bind _colorscheme_2 (Class|ColorSchemeInterface|GetColor(Message) (Game|GetGameMode) _colorscheme))
            (Default|SetAmmoCosmetic _asammo_cosmetic_interface (Utilities|Struct|MakeFAmmoCosmetics _colorscheme_2)))
          (:then_1
            (bind _ammocomponent (CallFunction|GetAmmoComponent _returnvalue_2))
            (Utilities|IsValid _ammocomponent
              (:Is%20Valid
                (Default|Initialize _ammocomponent _damagetag _basedamage)
                (Variables|/Game/PB/Blueprints/Gameplay/Ammo/BP_AmmoComponent.BP_AmmoComponent_C|SetAmmoTag _ammocomponent AmmoTag)
                (return _ammocomponent))
              (:Is%20Not%20Valid
                (Actor|DestroyActor _returnvalue_2)))))
        (else
          (Development|PrintString "BP_AmmoFactory::Invalid Ammo" :!label _label)))
      (else
        (goto _label)))
    (else
      (goto _label))))

(fn GetAmmoData
  (params (AmmoTag :type Gameplay%20Tag%20Structure))
  (bind _ammodata (Variables|Default|GetAmmoData))
  (bind (_value _returnvalue) (Utilities|Map|Find _ammodata AmmoTag))
  (return _returnvalue _value))