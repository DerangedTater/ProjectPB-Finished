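; BP_Property is a generic bounded gameplay value with give, take, affordability check and optional regeneration.
; Give and Take route through Adjust, which clamps Current between Min and Max, broadcasts OnAdjusted with the new amount and ratio, and returns the applied change.
; Initialize optionally fills to Max and, for a positive RegenPerSecond, starts a looping timer whose interval is the inverse of that rate, apparently driving DoRegen's single-point increments.
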(fn Give
  (params (Amount :type Float%20%28single-precision%29))
  (bind _adjustment (CallFunction|Adjust (+ (Variables|Default|GetCurrent) Amount)))
  (return _adjustment))

(fn Take
  (params (Amount :type Float%20%28single-precision%29))
  (bind _adjustment (CallFunction|Adjust (- (Variables|Default|GetCurrent) Amount)))
  (return (Math|Float|Absolute(Float) _adjustment)))

(fn Adjust
  (params (NewValue :type Float%20%28single-precision%29))
  (LocalVariables|SetLPrevious (Variables|Default|GetCurrent))
  (bind _output_get (Variables|Default|SetCurrent (Math|Float|Clamp(Float) NewValue (Variables|Default|GetMin) (Variables|Default|GetMax))))
  (Default|CallOnAdjusted _output_get (CallFunction|GetRatio))
  (return (- _output_get (LocalVariables|GetLPrevious))))

(fn Initialize
  (bind _regenpersecond (Variables|Default|GetRegenPerSecond))
  (Utilities|FlowControl|Sequence
    (:then_0
      (if (Variables|Default|GetbMaxOnStart)
        (CallFunction|Adjust (Variables|Default|GetMax))))
    (:then_1
      (if (> _regenpersecond 0.0)
        (Utilities|Time|SetTimerbyEvent (EventDispatchers|CreateEvent :!event DoRegen) (/ 1.0 _regenpersecond) true)))))

(fn CanTake
  (params (Amount :type Float%20%28single-precision%29))
  (return (>= (Variables|Default|GetCurrent) Amount)))

(fn DoRegen
  (CallFunction|Give 1.0))

(fn GetRatio
  (bind _max (Variables|Default|GetMax))
  (if (> _max 0.0)
    (return (/ (Variables|Default|GetCurrent) _max))
    (else
      (return 0.0))))