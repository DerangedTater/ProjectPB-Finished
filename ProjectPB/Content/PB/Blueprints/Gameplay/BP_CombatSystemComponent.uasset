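; Combat component that manages its owner's weapons, ammo and combat slots.
; Loadout tags become BP_WeaponSlot objects, pairing a factory-created weapon with BP_GameplayProperty ammo pools cached and shared by tag.
; Starting a slot delegates to it, and its pre-fire event arms that weapon, disarming the current one.
; Arming toggles weapons, snaps them between tag-found, cached equipped and unequipped components, and relays fire and ammo-cycle events.
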(fn GrantWeapon
  (params (WeaponTag :type Gameplay%20Tag%20Structure))
  (bind _weaponcomponent (Default|CreateWeapon (CallFunction|GetWeaponFactory) WeaponTag))
  (Utilities|IsValid _weaponcomponent
    (:Is%20Valid
      (Utilities|FlowControl|Sequence
        (:then_0
          (Variables|/Script/Engine.Actor|SetInstigator (Components|GetOwner _weaponcomponent) (Variables|/Script/Engine.Actor|GetInstigator (Components|GetOwner)))
          (bind _returnvalue (Utilities|Array|AddUnique (Variables|Hidden|GetWeapons) _weaponcomponent))
          ;[1 1 1] Arm if first added weapon
          (if (== _returnvalue 0)
            (Interface|ArmWeapon _returnvalue)))
        (:then_1
          (return _weaponcomponent))))))

(fn ArmWeapon
  (params (WeaponIndex :type Integer))
  (bind _weaponcomponent (CallFunction|GetWeaponbyIndex WeaponIndex))
  (if (!= WeaponIndex (Variables|Hidden|GetCurrentWeaponIndex))
    (if (Utilities|Array|IsValidIndex (Variables|Hidden|GetWeapons) WeaponIndex)
      (CallFunction|DisarmWeapon (Variables|Hidden|GetCurrentWeaponIndex))
      (Utilities|IsValid _weaponcomponent
        (:Is%20Valid
          (Default|EnableSelf _weaponcomponent)
          (Internal|HandleWeaponBinds _weaponcomponent true)
          (bind _equippedcomponent (CallFunction|GetEquippedComponent))
          (Transformation|AttachComponentToComponent (Components|GetOwner _weaponcomponent) _equippedcomponent (Variables|Config|GetEquippedSocketTag) "SnapToTarget" "SnapToTarget" "SnapToTarget" true)
          (Variables|Hidden|SetCurrentWeaponIndex WeaponIndex)
          (Default|CallOnAmmoCycled (Variables|/Game/PB/Blueprints/Gameplay/Weapon/BP_WeaponComponent.BP_WeaponComponent_C|GetAmmoToFire _weaponcomponent)))))))

(fn HandleWeaponBinds
  (params (WeaponComponent :type BP%20Weapon%20Component%20Object%20Reference) (bBind :type Boolean))
  (if bBind
    (EventDispatchers|BindEventtoOnFireFinished WeaponComponent (EventDispatchers|CreateEvent :!event HandleWeaponFireFinished))
    (else
      (EventDispatchers|UnbindEventfromOnFireFinished WeaponComponent (EventDispatchers|CreateEvent :!event HandleWeaponFireFinished)))))

(fn HandleWeaponFireFinished
  (params (bSuccess :type Boolean))
  (if bSuccess
    (Default|CallOnWeaponFired)
    (else
      (Default|CallOnWeaponFireFailed))))

(fn EquipWeapon
  (params (WeaponComponent :type BP%20Weapon%20Component%20Object%20Reference))
  (Transformation|AttachComponentToComponent (Components|GetOwner WeaponComponent) 0 "None" "KeepRelative" "KeepRelative" "KeepRelative" true))

(fn DisarmWeapon
  (params (WeaponIndex :type Integer))
  (bind _weaponcomponent (CallFunction|GetWeaponbyIndex WeaponIndex))
  (if (Utilities|Array|IsValidIndex (Variables|Hidden|GetWeapons) WeaponIndex)
    (Utilities|IsValid _weaponcomponent
      (:Is%20Valid
        (Utilities|FlowControl|Sequence
          (:then_0
            (if (== (CallFunction|GetCurrentWeapon) _weaponcomponent)
              (CallFunction|EmptyWeapon)))
          (:then_1
            (Default|DisableSelf _weaponcomponent)
            (Internal|HandleWeaponBinds _weaponcomponent false)
            (bind _unequippedcomponent (CallFunction|GetUnequippedComponent))
            (Transformation|AttachComponentToComponent (Components|GetOwner _weaponcomponent) _unequippedcomponent (Variables|Config|GetUnequippedSocketTag) "SnapToTarget" "SnapToTarget" "SnapToTarget" true)))))))

(fn GetCurrentWeapon
  (return (CallFunction|GetWeaponbyIndex (Variables|Hidden|GetCurrentWeaponIndex))))

(fn GetWeaponbyIndex
  (params (Index :type Integer))
  (bind _weapons (Variables|Hidden|GetWeapons))
  (if (Utilities|Array|IsValidIndex _weapons Index)
    (return (Utilities|Array|Get(acopy) _weapons Index))))

(fn EmptyWeapon
  (Variables|Hidden|SetCurrentWeaponIndex -1))

(fn GetAmmoProperty
  (params (AmmoIndex :type Integer))
  (bind _ammocached (Variables|Hidden|GetAmmoCached))
  (bind _ammoorder (Variables|Hidden|GetAmmoOrder))
  (bind _output (Utilities|Array|Get(acopy) _ammoorder AmmoIndex))
  (bind (_value _returnvalue) (Utilities|Map|Find _ammocached _output))
  (if (Utilities|Array|IsValidIndex _ammoorder AmmoIndex)
    (if _returnvalue
      (return _value))))

(fn GetCurrentAmmoProperty
  (return (CallFunction|GetAmmoProperty (Variables|Hidden|GetCurrentAmmoIndex))))

(fn GetEquippedComponent
  (bind _returnvalue (Components|GetOwner))
  (bind _equippedtag (Variables|Config|GetEquippedTag))
  (bind _returnvalue_2 (Actor|GetComponentsbyTag _returnvalue "/Script/Engine.SceneComponent" _equippedtag))
  (Utilities|IsValid (Variables|Hidden|GetEquippedComponent)
    (:Is%20Valid
      (return (Variables|Hidden|GetEquippedComponent)))
    (:Is%20Not%20Valid
      (if (> (Utilities|Array|Length _returnvalue_2) 0)
        (bind _output_get (Variables|Hidden|SetEquippedComponent (Utilities|Array|Get(acopy) _returnvalue_2)))
        (return _output_get)))))

(fn GetUnequippedComponent
  (bind _returnvalue (Components|GetOwner))
  (bind _unequippedtag (Variables|Config|GetUnequippedTag))
  (bind _returnvalue_2 (Actor|GetComponentsbyTag _returnvalue "/Script/Engine.SceneComponent" _unequippedtag))
  (Utilities|IsValid (Variables|Hidden|GetUnequippedComponent)
    (:Is%20Valid
      (return (Variables|Hidden|GetUnequippedComponent)))
    (:Is%20Not%20Valid
      (if (> (Utilities|Array|Length _returnvalue_2) 0)
        (bind _output_get (Variables|Hidden|SetUnequippedComponent (Utilities|Array|Get(acopy) _returnvalue_2)))
        (return _output_get)))))

(fn GiveAmmo
  (params (AmmoTag :type Gameplay%20Tag%20Structure) (Amount :type Float%20%28single-precision%29))
  (bind _ammocached (Variables|Hidden|GetAmmoCached))
  (bind (_value _returnvalue) (Utilities|Map|Find _ammocached AmmoTag))
  (bind _bisvalid (CallFunction|GetAmmoData AmmoTag))
  (if _bisvalid
    (if _returnvalue
      (Default|Give _value Amount))))

(fn SetLoadouts
  (params (LoadoutTag :type Array%20of%20Gameplay%20Tag%20Structures))
  (for _array_element LoadoutTag
    (bind _slot (CallFunction|SetupSlotLoadout _array_element))
    (Utilities|Array|Add (Variables|Default|GetSlots) _slot))
  (return (Variables|Default|GetSlots)))

(fn InitAmmo
  (params (AmmoLoadout :type F%20Ammo%20Loadout%20Structure))
  (bind _ammocached (Variables|Hidden|GetAmmoCached))
  (bind (_value _returnvalue) (Utilities|Map|Find _ammocached (.ammotype AmmoLoadout)))
  (Utilities|FlowControl|Sequence
    (:then_0
      (if _returnvalue
        (LocalVariables|SetLAmmoCache _value)
        (else
          (bind _returnvalue_2 (Game|ConstructObjectfromClass "/Game/PB/Blueprints/Gameplay/Properties/BP_GameplayProperty.BP_GameplayProperty_C" self))
          (bind _output_get (LocalVariables|SetLAmmoCache _returnvalue_2))
          (Variables|/Game/PB/Blueprints/Gameplay/Properties/BP_Property.BP_Property_C|SetRegenPerSecond _output_get (.regenpersecond AmmoLoadout))
          (Default|Initialize _output_get)
          (Variables|/Game/PB/Blueprints/Gameplay/Properties/BP_GameplayProperty.BP_GameplayProperty_C|SetGameplayTag _output_get (.ammotype AmmoLoadout))
          (Utilities|Map|Add (Variables|Hidden|GetAmmoCached) (.ammotype AmmoLoadout) _output_get)
          (bind _returnvalue_3 (Utilities|Array|AddUnique (Variables|Hidden|GetAmmoOrder) (.ammotype AmmoLoadout)))
          (if (== _returnvalue_3 0)
            (Variables|Hidden|SetCurrentAmmoIndex 0)))))
    (:then_1
      (Variables|/Game/PB/Blueprints/Gameplay/Properties/BP_Property.BP_Property_C|SetMax (LocalVariables|GetLAmmoCache) (.capacity AmmoLoadout))
      (Default|Adjust (LocalVariables|GetLAmmoCache) (.startingamount AmmoLoadout)))
    (:then_2
      (return (LocalVariables|GetLAmmoCache)))))

(fn SetupStartingWeapons
  (params (StartingWeaponTags :type Array%20of%20Gameplay%20Tag%20Structures))
  (bind _output_get (Variables|Hidden|SetStartingWeaponTags StartingWeaponTags))
  (for _array_element _output_get
    (Interface|GrantWeapon _array_element)))

(fn DestroyAllOwned
  (for _array_element (Variables|Hidden|GetWeapons)
    (Actor|DestroyActor (Components|GetOwner _array_element))))

(fn CurrentWeaponTag)

(fn SetupSlotLoadout
  (params (LoadoutTag :type Gameplay%20Tag%20Structure))
  (bind _loadoutdata (CallFunction|GetLoadout LoadoutTag))
  (bind _weapon (Interface|GrantWeapon (.weapontag _loadoutdata)))
  (Utilities|IsValid _weapon
    (:Is%20Valid
      (bind _returnvalue (Game|ConstructObjectfromClass "/Game/PB/Blueprints/Gameplay/CombatSlot/BP_WeaponSlot.BP_WeaponSlot_C" self))
      (bind _output_get (Variables|/Game/PB/Blueprints/Gameplay/CombatSlot/BP_WeaponSlot.BP_WeaponSlot_C|SetWeapon _returnvalue _weapon))
      (for _array_element (.ammo _loadoutdata)
        (bind _ammo (CallFunction|InitAmmo _array_element))
        (Utilities|Array|AddUnique (LocalVariables|GetLAmmoForSlot) _ammo))
      (bind _output_get_2 (Variables|/Game/PB/Blueprints/Gameplay/CombatSlot/BP_WeaponSlot.BP_WeaponSlot_C|SetAvailableAmmo _returnvalue (LocalVariables|GetLAmmoForSlot)))
      (if (> (Utilities|Array|Length _output_get_2) 0)
        (Default|UpdateAmmo _output_get (Utilities|Array|Get(acopy) _output_get_2))
        (EventDispatchers|BindEventtoOnPreFireWeapon _returnvalue (EventDispatchers|CreateEvent :!event HandlePreFireWeapon))
        (EventDispatchers|BindEventtoOnAmmoCycled _returnvalue (EventDispatchers|CreateEvent :!event HandleAmmoCycled))
        (return _returnvalue)))))

(fn StartCombatSlot
  (params (Index :type Integer))
  (bind _slots (Variables|Default|GetSlots))
  (if (Utilities|Array|IsValidIndex _slots Index)
    (Default|StartCombatSlot (Utilities|Array|Get(acopy) _slots Index))))

(fn StopCombatSlot
  (params (Index :type Integer))
  (bind _slots (Variables|Default|GetSlots))
  (if (Utilities|Array|IsValidIndex _slots Index)
    (Default|StopCombatSlot (Utilities|Array|Get(acopy) _slots Index))))

(fn HandlePreFireWeapon
  (params (Weapon :type BP%20Weapon%20Component%20Object%20Reference))
  (bind _weapons (Variables|Hidden|GetWeapons))
  (bind _returnvalue (Utilities|Array|FindItem _weapons Weapon))
  (if (>= _returnvalue 0)
    (Interface|ArmWeapon _returnvalue)))

(fn HandleAmmoCycled
  (params (AmmoProperty :type BP%20Gameplay%20Property%20Object%20Reference))
  (Default|CallOnAmmoCycled AmmoProperty))