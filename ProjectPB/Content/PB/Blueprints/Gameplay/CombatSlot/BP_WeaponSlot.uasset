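; BP_WeaponSlot is a combat slot that controls a weapon and the ammo types available to it.
; Starting the slot raises a pre-fire event and starts the weapon firing, and stopping it halts fire.
; Cycling options steps through available ammo with wraparound in either direction, updates the weapon and broadcasts the change.
; GetData returns the weapon's shot interval multiplied by the selected ammo's Current value.
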(event EventStartCombatSlot
  (Default|CallOnPreFireWeapon (Variables|Default|GetWeapon))
  (CallFunction|StartWeapon))

(event EventStopCombatSlot
  (CallFunction|StopWeapon))

(event EventCycleCombatSlotOptions
  (params (Forward :type Boolean))
  (CallFunction|CycleAmmo Forward))

(fn CycleAmmo
  (params (Increment :type Boolean))
  (bind _weapon (Variables|Default|GetWeapon))
  (Variables|Default|SetCurrentAmmoIndex (CallFunction|CycleAmmoIndex Increment))
  (Default|CallOnPreFireWeapon _weapon)
  (Default|UpdateAmmo _weapon (Utilities|Array|Get(acopy) (Variables|Default|GetAvailableAmmo) (Variables|Default|GetCurrentAmmoIndex)))
  (Default|CallOnAmmoCycled (Utilities|Array|Get(acopy) (Variables|Default|GetAvailableAmmo) (Variables|Default|GetCurrentAmmoIndex))))

(fn StartWeapon
  (bind _weapon (Variables|Default|GetWeapon))
  (Utilities|IsValid _weapon
    (:Is%20Valid
      (Default|StartFiring _weapon))))

(fn StopWeapon
  (bind _weapon (Variables|Default|GetWeapon))
  (Utilities|IsValid _weapon
    (:Is%20Valid
      (Default|StopFiring _weapon))))

(fn CycleAmmoIndex
  (params (Forward :type Boolean))
  (bind _currentammoindex (Variables|Default|GetCurrentAmmoIndex))
  (bind _availableammo (Variables|Default|GetAvailableAmmo))
  (bind _returnvalue (Utilities|Array|LastIndex _availableammo))
  (bind _returnvalue_2 (- _currentammoindex 1))
  (bind _returnvalue_3 (+ _currentammoindex 1))
  (if Forward
    (if (> _returnvalue_3 _returnvalue)
      (return 0)
      (else
        (return _returnvalue_3)))
    (elif (< _returnvalue_2 0)
      (return _returnvalue)
      (else
        (return _returnvalue_2)))))

(fn GetData
  (bind _availableammo (Variables|Default|GetAvailableAmmo))
  (bind _currentammoindex (Variables|Default|GetCurrentAmmoIndex))
  (if (Utilities|Array|IsValidIndex _availableammo _currentammoindex)
    (return (* (/ 1.0 (Variables|/Game/PB/Blueprints/Gameplay/Weapon/BP_WeaponComponent.BP_WeaponComponent_C|GetShotPerSecond (Variables|Default|GetWeapon))) (Variables|/Game/PB/Blueprints/Gameplay/Properties/BP_Property.BP_Property_C|GetCurrent (Utilities|Array|Get(acopy) _availableammo _currentammoindex))))))