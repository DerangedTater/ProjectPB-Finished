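; BP_Weapon_Factory spawns weapons by tag from data defined in DT_Weapons.
; On BeginPlay it caches every table row in a map keyed by WeaponTag for validated lookup.
; CreateWeapon spawns the row's weapon type, applies the game mode's color scheme through WeaponCosmeticInterface, then tags and returns its weapon component.
; Failed cosmetic casts skip only coloring, while actors lacking a valid weapon component are destroyed.
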(event EventBeginPlay
  (CallFunction|CacheWeapons))

(fn ConstructionScript)

(fn CacheWeapons
  (bind _outrownames (DataTable|GetDataTableRowNames "/Game/PB/Data/Weapons/DT_Weapons.DT_Weapons"))
  (for _array_element _outrownames
    (bind _returnvalue (Utilities|GetDataTableRow "/Game/PB/Data/Weapons/DT_Weapons.DT_Weapons" _array_element)
      (:then
        (Utilities|Map|Add (Variables|Default|GetWeaponCache) (.WeaponTag (Utilities|Struct|BreakFWeaponData _returnvalue)) _returnvalue)))))

(fn GetWeaponData
  (params (WeaponTag :type Gameplay%20Tag%20Structure))
  (bind _weaponcache (Variables|Default|GetWeaponCache))
  (bind (_value _returnvalue) (Utilities|Map|Find _weaponcache WeaponTag))
  (if _returnvalue
    (return _value true)
    (else
      (return "" false))))

(fn CreateWeapon
  (params (WeaponTag :type Gameplay%20Tag%20Structure))
  (bind (_weapondata _isvalid) (CallFunction|GetWeaponData WeaponTag))
  (if _isvalid
    (bind _returnvalue (Game|SpawnActorfromClass (Utilities|GetClassDefaults (.weapontype _weapondata)) (Math|Transform|MakeTransform "0, 0, 0" "0, 0, 0" "1,1,1") "Undefined" 0 0))
    (Utilities|FlowControl|Sequence
      (:then_0
        (bind _asweapon_cosmetic_interface (Utilities|Casting|CastToWeaponCosmeticInterface _returnvalue))
        (bind _colorscheme (Class|ColorSchemeInterface|GetColor(Message) (Game|GetGameMode) (.colorscheme _weapondata)))
        (Default|SetWeaponCosmetic _asweapon_cosmetic_interface (Utilities|Struct|MakeFWeaponCosmetic _colorscheme)))
      (:then_1
        (bind _weaponcomponent (CallFunction|GetWeaponComponent _returnvalue))
        (Utilities|IsValid _weaponcomponent
          (:Is%20Valid
            (Variables|/Game/PB/Blueprints/Gameplay/Weapon/BP_WeaponComponent.BP_WeaponComponent_C|SetWeaponTag _weaponcomponent WeaponTag)
            (return _weaponcomponent))
          (:Is%20Not%20Valid
            (Actor|DestroyActor _returnvalue)))))
    (else
      (Development|PrintString "Attempt to create invalid weapon type." false))))