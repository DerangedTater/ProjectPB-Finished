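; Behavior tree task that starts or stops weapon fire on an AI pawn, depending on its Start flag.
; It drives the first slot of the pawn's combat system component.
; When starting, it writes a random duration, capped by the slot's data, to the RemainingShotTime blackboard key.
; It finishes successfully right away, but never calls FinishExecute if the component or slot is missing.
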(event EventReceiveExecuteAI
  (params (OwnerController :type AI%20Controller%20Object%20Reference) (ControlledPawn :type Pawn%20Object%20Reference))
  (bind _combatsystem (CallFunction|GetCombatSystemComponent ControlledPawn))
  (Utilities|IsValid _combatsystem
    (:Is%20Valid
      (if (Utilities|Array|IsValidIndex (Variables|/Game/PB/Blueprints/Gameplay/BP_CombatSystemComponent.BP_CombatSystemComponent_C|GetSlots _combatsystem))
        (if (Variables|Default|GetbStart)
          (Default|StartCombatSlot (Utilities|Array|Get(acopy) (Variables|/Game/PB/Blueprints/Gameplay/BP_CombatSystemComponent.BP_CombatSystemComponent_C|GetSlots _combatsystem)))
          (bind _remainingshottimer (Default|GetData (Utilities|Array|Get(acopy) (Variables|/Game/PB/Blueprints/Gameplay/BP_CombatSystemComponent.BP_CombatSystemComponent_C|GetSlots _combatsystem))))
          (Class|BTFunctionLibrary|SetBlackboardValueasFloat (Variables|Default|GetRemainingShotTime) (Math|Random|RandomFloatinRange 1.0 _remainingshottimer))
          (else
            (Default|StopCombatSlot (Utilities|Array|Get(acopy) (Variables|/Game/PB/Blueprints/Gameplay/BP_CombatSystemComponent.BP_CombatSystemComponent_C|GetSlots _combatsystem)))))
        (AI|BehaviorTree|FinishExecute true)))))