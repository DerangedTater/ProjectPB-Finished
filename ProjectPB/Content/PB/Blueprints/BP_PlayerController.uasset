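; Player controller that links the possessed character to the HUD through a character listener object.
; Shortly after BeginPlay, it caches the custom HUD, constructs a BP_CharacterListener, initializes it with the controlled PBCharacter, and passes it to the HUD.
; The link is made once after a brief fixed delay, with no handling for later possession changes.
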(event EventBeginPlay
  (Utilities|FlowControl|Delay 0.2)
  (bind _ascustom_hud (Utilities|Casting|CastToCustom_HUD (HUD|GetHUD)))
  (Variables|Default|SetHUD _ascustom_hud)
  (bind _returnvalue (Game|ConstructObjectfromClass "/Game/PB/UI/BP_CharacterListener.BP_CharacterListener_C" self))
  (bind _aspbcharacter (Utilities|Casting|CastToPBCharacter (Pawn|GetControlledPawn)))
  (Default|Initialize _returnvalue _aspbcharacter)
  (Default|ReceiveCharacterListener (Variables|Default|GetHUD) _returnvalue))

(fn ConstructionScript)